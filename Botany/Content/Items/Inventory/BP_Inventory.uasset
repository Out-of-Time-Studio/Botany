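; BP_Inventory stores items as a list of item and quantity entries, with AddItem handling stacking.
; AddItem loops over the entries and, on the first match, increments its quantity, closes a Gate and breaks.
; The Gate, entered after the loop, lets only unmatched items through to be added with quantity one.
; The ItemAdded call fires only on that new-entry path, not when a stack grows.
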(fn AddItem
  (params (Item :type BP%20Item%20Object%20Reference))
  (bind _items (Variables|Default|GetItems))
  (bind (_array_element _array_index) (Utilities|Array|ForEachLoopwithBreak _items :!label _label)
    (:LoopBody
      (if (Default|Compare (.item _array_element) Item)
        (Math|Integer|IncrementInt (.quantity (Utilities|Array|Get(acopy) _items _array_index))
          (:%20%20
            (Utilities|FlowControl|Sequence
              (:then_0
                (goto _label_2 Close))
              (:then_1
                (goto _label Break)))))))
    (:Completed
      (Utilities|FlowControl|Gate false :!label _label_2
        (:Exit
          (Utilities|Array|AddUnique (Variables|Default|GetItems) (Utilities|Struct|MakeInventory_Item Item 1))
          (Default|CallItemAdded (Utilities|Struct|MakeInventory_Item Item 1)))))))