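; Blueprint function library of general-purpose math helpers for floats and integers.
; In-place add, subtract, multiply and divide functions write to a by-ref value and return the result, though DivideValueInt actually multiplies.
; Average and weighted PonderAverage accumulate sums through AddValue, with no guard against dividing by zero.
; Further helpers truncate decimals, compute a ratio or percentage, and test for non-negative numbers.
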(fn Average
  (params (Floats :type Array%20of%20Floats%20%28double-precision%29))
  (for _array_element Floats
    (CallFunction|AddValue (LocalVariables|GetSum) _array_element))
  (return (/ (LocalVariables|GetSum) (Utilities|Array|Length Floats))))

(fn AddValue
  (params (Value :type Float%20%28double-precision%29%20%28by%20ref%29) (Add :type Float%20%28double-precision%29))
  (bind _returnvalue (+ Value Add))
  (|SetBy-RefVar Value _returnvalue)
  (return _returnvalue))

(fn AddValueInt
  (params (Value :type Integer%20%28by%20ref%29) (Add :type Integer))
  (bind _returnvalue (+ Value Add))
  (|SetBy-RefVar Value _returnvalue)
  (return _returnvalue))

(fn PonderAverage
  (params (Pondered%20Floats :type Array%20of%20Floats%20Tuple%20Structure))
  (for _array_element Pondered%20Floats
    (CallFunction|AddValue (LocalVariables|GetSum) (* (.a _array_element) (.b _array_element)))
    (CallFunction|AddValue (LocalVariables|GetPonderSum) (.b _array_element)))
  (return (/ (LocalVariables|GetSum) (LocalVariables|GetPonderSum))))

(fn SubstractValue
  (params (Value :type Float%20%28double-precision%29%20%28by%20ref%29) (Substract :type Float%20%28double-precision%29))
  (bind _returnvalue (- Value Substract))
  (|SetBy-RefVar Value _returnvalue)
  (return _returnvalue))

(fn SubstractValueInt
  (params (Value :type Integer%20%28by%20ref%29) (Substract :type Integer))
  (bind _returnvalue (- Value Substract))
  (|SetBy-RefVar Value _returnvalue)
  (return _returnvalue))

(fn MultiplyValue
  (params (Value :type Float%20%28double-precision%29%20%28by%20ref%29) (Multiply :type Float%20%28double-precision%29))
  (bind _returnvalue (* Value Multiply))
  (|SetBy-RefVar Value _returnvalue)
  (return _returnvalue))

(fn MultiplyValueInt
  (params (Value :type Integer%20%28by%20ref%29) (Multiply :type Integer))
  (bind _returnvalue (* Value Multiply))
  (|SetBy-RefVar Value _returnvalue)
  (return _returnvalue))

(fn DivideValue
  (params (Value :type Float%20%28double-precision%29%20%28by%20ref%29) (Divide :type Float%20%28double-precision%29))
  (bind _returnvalue (/ Value Divide))
  (|SetBy-RefVar Value _returnvalue)
  (return _returnvalue))

(fn DivideValueInt
  (params (Value :type Integer%20%28by%20ref%29) (Divide :type Integer))
  (bind _returnvalue (* Value Divide))
  (|SetBy-RefVar Value _returnvalue)
  (return _returnvalue))

(fn TruncateDecimals
  (params (Number :type Float%20%28double-precision%29) (Decimals :type Integer))
  (bind _returnvalue (Math|Conversions|ToFloat(Integer) Decimals))
  (bind _returnvalue_2 (Math|Float|Power 1e+01 _returnvalue))
  (return (/ (Math|Conversions|ToFloat(Integer) (Math|Float|Truncate (* Number _returnvalue_2))) _returnvalue_2)))

(fn Percent
  (params (Numerator :type Float%20%28double-precision%29) (Denumerator :type Float%20%28double-precision%29) (As%20Percent :type Boolean))
  (return (* (/ Numerator Denumerator) (Math|Float|SelectFloat 1e+02 1.0 As%20Percent))))

(fn IsPositive?
  (params (Number :type Float%20%28double-precision%29))
  (return (>= Number 0.0)))