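; Blueprint function library of text utilities for joining texts, measuring text length and formatting numbers as padded strings.
; ConcatText joins two texts with or without a separating space, and GetLength counts characters through a string conversion.
; FormatNumber puts the truncated integer or decimal-limited value between zero padding built by two looping helper graphs, one for leading and one for trailing digits.
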(fn ConcatText
  (params (Text1 :type Text) (Text2 :type Text) (SeperateLines :type Boolean))
  (return (select SeperateLines (Utilities|Text|FormatText "{0}
{1}" Text1 Text2) (Utilities|Text|FormatText "{0}{1}" Text1 Text2))))

(fn GetLength
  (params (Text :type Text))
  (return (Utilities|String|Len (Utilities|String|ToString(Text) Text))))

(fn FormatNumber
  (params (Number :type Float%20%28double-precision%29) (Integer? :type Boolean) (digits%20in%20front%20comma :type Integer) (digits%20behind%20comma :type Integer))
  (bind _frontstring (|DigitsinFront Number digits%20in%20front%20comma)
    (:Completed
      (bind _back_string (|DigitsatBack Number digits%20behind%20comma)
        (:Completed
          (return (Utilities|String|Append _frontstring (Utilities|String|SelectString (Utilities|String|ToString(Integer) (Math|Float|Truncate Number)) (Utilities|String|ToString(Float) (CallFunction|TruncateDecimals Number digits%20behind%20comma)) Integer?) _back_string)))))))