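; Blueprint function library of vector math helpers for getting angles and directions relative to a component.
; GetRelativePitch and GetRelativeYaw project a vector onto the plane normal to the reference's right or up axis, then take its angle from forward.
; A cross product dotted with that axis supplies the sign of each angle.
; GetDownVector returns a component's negated up vector.
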(fn GetRelativePitch
  (params (Reference :type Scene%20Component%20Object%20Reference) (InVector :type Vector))
  (bind _returnvalue (Math|Vector|GetRightVector Reference))
  (bind _returnvalue_2 (Math|Vector|GetForwardVector Reference))
  (bind _returnvalue_3 (Math|Vector|ProjectVectorontoPlane InVector _returnvalue))
  (bind _returnvalue_4 (Math|Vector|Normalize _returnvalue_3))
  (return (* (Class|KismetMathLibrary|DegAcos (Math|Vector|DotProduct _returnvalue_2 _returnvalue_4)) (Math|Float|SelectFloat -1.0 1.0 (<= (Math|Vector|DotProduct (Math|Vector|CrossProduct _returnvalue_4 _returnvalue_2) _returnvalue) 0.0)))))

(fn GetRelativeYaw
  (params (Reference :type Scene%20Component%20Object%20Reference) (InVector :type Vector))
  (bind _returnvalue (Math|Vector|GetUpVector Reference))
  (bind _returnvalue_2 (Math|Vector|GetForwardVector Reference))
  (bind _returnvalue_3 (Math|Vector|ProjectVectorontoPlane InVector _returnvalue))
  (bind _returnvalue_4 (Math|Vector|Normalize _returnvalue_3))
  (return (* (Class|KismetMathLibrary|DegAcos (Math|Vector|DotProduct _returnvalue_2 _returnvalue_4)) (Math|Float|SelectFloat 1.0 -1.0 (<= (Math|Vector|DotProduct (Math|Vector|CrossProduct _returnvalue_4 _returnvalue_2) _returnvalue) 0.0)))))

(fn GetDownVector
  (params (Component :type Scene%20Component%20Object%20Reference))
  (return (* (Math|Vector|GetUpVector Component) -1.0)))